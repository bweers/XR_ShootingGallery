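; BP_AlienRoundTriggerTarget is a shootable target that starts a round on the alien target manager when knocked down.
; KnockDown calls StartRound, disables collision, plays a pitch-tipping timeline with a hit sound, then destroys the actor after a short delay.
; BeginPlay reverses that timeline from its end to raise the target.
; Sideways movement and direction-flip functions exist, but the looping movement timer is left unconnected.
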(event `UpdatePosition`
  (`self.K2_AddActorWorldOffset` (* (`self.GetActorRightVector`) (`self.Speed`))))

(event `/Game/Targets/BPI_Targets.KnockDown`
  (params (CountsForPoints :type Boolean))
  (`|ExecutionSequence`
    (:`then_0`
      (`/Game/Targets/BP_AlienTargetManager1.StartRound` (`self.alientmanagref`)))
    (:`then_1`
      (`PrimitiveComponent.SetCollisionEnabled` (`self.Collider`) "NoCollision")
      (bind (_direction _yrotation) (`Timeline|KnockDownAnimTimeline` :!label _label)
        (:`Update`
          (`self.K2_SetActorRotation` (`KismetMathLibrary.MakeRotator` 0.0 _yrotation)))))
    (:`then_2`
      (`KismetSystemLibrary.Delay` 0.2)
      (`self.K2_DestroyActor`))
    (:`then_3`
      (`GameplayStatics.PlaySoundAtLocation` "/Game/Audio/target/CUE_target_hitping.CUE_target_hitping" (`self.K2_GetActorLocation`) (struct) 1.0 1.0 0.0 null null null))))

(event `self.ReceiveBeginPlay`
  (goto _label :!via `ReverseFromEnd`))

(fn `SwitchDirection`
  (set `self.Speed` (* (`self.Speed`) -1.0)))

(fn `UserConstructionScript`)
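; BP_MovieSelect is the target manager for a shooting-gallery game, running timed rounds, target spawning and streak-based scoring.
; StartRound starts looping countdown and spawn timers; EndRound clears them, knocks down targets and advances the act manager.
; Targets use round-specific meshes and spawn from either side of two rows, capped by overlap counts.
; It also spawns movie, round and thanks targets, while AddPoints multiplies points by streak and occasionally triggers mascot reactions.
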(event `Spawn Movie Target`
  (`KismetSystemLibrary.Delay` 0.35)
  (`|SpawnActorFromClass` "/Game/Targets/BP_CoolwaterTrigger.BP_CoolwaterTrigger_C" (`SceneComponent.K2_GetComponentToWorld` (`self.Left Upper SpawnPoint`)) "Undefined" "OverrideRootScale" null 0.35 self null)
  (`KismetSystemLibrary.Delay` 0.35)
  (`|SpawnActorFromClass` "/Game/Targets/BP_MartianTrigger1.BP_MartianTrigger1_C" (`SceneComponent.K2_GetComponentToWorld` (`self.Left Lower SpawnPoint`)) "Undefined" "OverrideRootScale" null 0.35 self null))

(event `SpawnTarget`
  (bind _targets_act1 (`self.Targets_Act1`))
  (bind _targets_act2 (`self.Targets_Act2`))
  (bind _targets_act3 (`self.Targets_Act3`))
  ;[0.09896 0.09896 0.09896] Target Spawning
  (`self.UpdateNumberOfTargets`)
  (`self.ChooseSpawnPoint`)
  (if (not (`self.RowsFull`))
    (switch `int` (`self.CurrentRound`)
      (:`1`
        (bind _returnvalue (`|SpawnActorFromClass` "/Game/Targets/BP_Target.BP_Target_C" (`KismetMathLibrary.MakeTransform` (+ (`self.SpawnCoordinate`) (`KismetMathLibrary.MakeVector` (`KismetMathLibrary.RandomFloatInRange` -5.0 1.0)))) "Undefined" "OverrideRootScale" null (`KismetMathLibrary.RandomFloatInRange` (`self.TargetSpeedMin`) (`self.TargetSpeedMax`)) self (`|GetArrayItem` _targets_act1 (`KismetMathLibrary.RandomIntegerInRange` 0 (- (`KismetArrayLibrary.Array_Length` _targets_act1) 1))) null))
        (if (`self.FlippedDirection`)
          (`/Game/Targets/BP_Target.SwitchDirection` _returnvalue)))
      (:`2`
        (bind _returnvalue_2 (`|SpawnActorFromClass` "/Game/Targets/BP_Target.BP_Target_C" (`KismetMathLibrary.MakeTransform` (+ (`self.SpawnCoordinate`) (`KismetMathLibrary.MakeVector` (`KismetMathLibrary.RandomFloatInRange` -5.0 1.0)))) "Undefined" "OverrideRootScale" null (`KismetMathLibrary.RandomFloatInRange` (`self.TargetSpeedMin`) (`self.TargetSpeedMax`)) self (`|GetArrayItem` _targets_act2 (`KismetMathLibrary.RandomIntegerInRange` 0 (- (`KismetArrayLibrary.Array_Length` _targets_act2) 1))) null))
        (if (`self.FlippedDirection`)
          (`/Game/Targets/BP_Target.SwitchDirection` _returnvalue_2)))
      (:`3`
        (bind _returnvalue_3 (`|SpawnActorFromClass` "/Game/Targets/BP_Target.BP_Target_C" (`KismetMathLibrary.MakeTransform` (+ (`self.SpawnCoordinate`) (`KismetMathLibrary.MakeVector` (`KismetMathLibrary.RandomFloatInRange` -5.0 1.0)))) "Undefined" "OverrideRootScale" null (`KismetMathLibrary.RandomFloatInRange` (`self.TargetSpeedMin`) (`self.TargetSpeedMax`)) self (`|GetArrayItem` _targets_act3 (`KismetMathLibrary.RandomIntegerInRange` 0 (- (`KismetArrayLibrary.Array_Length` _targets_act3) 1))) null))
        (if (`self.FlippedDirection`)
          (`/Game/Targets/BP_Target.SwitchDirection` _returnvalue_3))))))

(event `SpawnRoundTarget`
  (`KismetSystemLibrary.Delay` 0.35)
  (`|SpawnActorFromClass` "/Game/Targets/BP_RoundTriggerTarget.BP_RoundTriggerTarget_C" (`SceneComponent.K2_GetComponentToWorld` (`self.RoundTriggerTarget SpawnPoint`)) "Undefined" "OverrideRootScale" null 0.35 self null))

(event `SpawnThanksTarget`
  (`KismetSystemLibrary.Delay` 0.0)
  (`|SpawnActorFromClass` "/Game/Targets/BP_ThanksTarget.BP_ThanksTarget_C" (`SceneComponent.K2_GetComponentToWorld` (`self.RoundTriggerTarget SpawnPoint`)) "Undefined" "OverrideRootScale" null 0.0 self null))

(event `StreakTimer`
  ;[0.09896 0.09896 0.09896] Streak Timer
  (set `self.InStreak` false)
  (set `self.StreakCounter` 0 :!label _label))

(event `EndStreak`
  ;[0.09896 0.09896 0.09896] Streak Timer
  (set `self.InStreak` false)
  (`KismetSystemLibrary.K2_ClearAndInvalidateTimerHandle` (`self.StreakTimerRef`))
  (goto _label))

(event `StartRound`
  ;[0.09896 0.09896 0.09896] Rounds
  (set `self.RoundTimespan` (`KismetMathLibrary.MakeTimespan` 0 0 1 20))
  (`/Engine/EditorBlueprintResources/StandardMacros.IncrementInt` (`self.CurrentRound`)
    (:`  `
      (bind _returnvalue (`KismetSystemLibrary.K2_SetTimerDelegate` (`|CreateDelegate` :!event `RoundTimer`) 0.1 true))
      (set `self.RoundTimerRef` _returnvalue)
      (bind _returnvalue_2 (`KismetSystemLibrary.K2_SetTimerDelegate` (`|CreateDelegate` :!event `SpawnTarget`) 0.7 true))
      (set `self.SpawnTargetTimerRef` _returnvalue_2)
      (`KismetSystemLibrary.PrintString` "ROUND LIVE" true true (struct :`R` 0.277924 :`G` 1.0 :`A` 1.0) 10.0)
      (`GameplayStatics.PlaySound2D` "/Game/Audio/round/round_start_Cue.round_start_Cue" 1.0 1.0 0.0 null null))))

(event `EndRound`
  ;[0.09896 0.09896 0.09896] Rounds
  (`KismetSystemLibrary.K2_ClearAndInvalidateTimerHandle` (`self.RoundTimerRef`))
  (`KismetSystemLibrary.K2_ClearAndInvalidateTimerHandle` (`self.SpawnTargetTimerRef`))
  (`KismetSystemLibrary.PrintString` "TIMERS CLEARED")
  (bind _outactors (`GameplayStatics.GetAllActorsOfClass` "/Game/Targets/BP_Target.BP_Target_C"))
  (for _array_element _outactors
    (message `/Game/Targets/BPI_Targets.KnockDown` _array_element false))
  (`/Game/ActManager.Start Next Act` (`self.ActManagerRef`))
  (`GameplayStatics.PlaySound2D` "/Game/Audio/round/round_end_Cue.round_end_Cue" 1.0 1.0 0.0 null null))

(event `RoundTimer`
  ;[0.09896 0.09896 0.09896] Rounds
  (bind _output_get (set `self.RoundTimespan` (- (`self.RoundTimespan`) (`KismetMathLibrary.MakeTimespan` 0 0 0 0 100))))
  (if (<= _output_get (`KismetMathLibrary.MakeTimespan` 0))
    (`self.EndRound`))
  (bind (_days _hours _minutes _seconds) (`KismetMathLibrary.BreakTimespan` _output_get))
  (set `self.RoundTimerString` (`KismetStringLibrary.Concat_StrStr` (`KismetStringLibrary.Right` (`KismetStringLibrary.Conv_IntToString` _minutes) 1) ":" (`KismetStringLibrary.Conv_IntToString` _seconds))))

(fn `AddPoints`
  (params (PointValue :type Integer))
  (if (`self.InStreak`)
    (`KismetSystemLibrary.K2_ClearAndInvalidateTimerHandle` (`self.StreakTimerRef`))
    (bind _returnvalue (`KismetSystemLibrary.K2_SetTimerDelegate` (`|CreateDelegate` :!event `StreakTimer`) 2.5))
    (set `self.StreakTimerRef` _returnvalue)
    (`/Engine/EditorBlueprintResources/StandardMacros.IncrementInt` (`self.StreakCounter`)
      (:`  `
        (`|ExecutionSequence`
          (:`then_0`
            (if (== (`self.StreakCounter`) 6)
              (if (== (`KismetMathLibrary.RandomIntegerInRange` 0 2) 0)
                (`/Game/Mascot/BP_Mascot.React_GoodShot` (`self.MascotRef`)))))
          (:`then_1`
            (bind _output_get (set `self.Points` (+ (`self.Points`) (* PointValue (`self.StreakCounter`))) :!label _label))))))
    (else
      (set `self.InStreak` true)
      (bind _returnvalue_2 (`KismetSystemLibrary.K2_SetTimerDelegate` (`|CreateDelegate` :!event `StreakTimer`) 2.5))
      (set `self.StreakTimerRef` _returnvalue_2)
      (set `self.StreakCounter` 1)
      (goto _label))))

(fn `ChooseSpawnPoint`
  (set `self.RowsFull` false)
  (if (== (`KismetMathLibrary.RandomIntegerInRange` 0 1) 0)
    (if (>= (`self.UpperRowTargetsCount`) (`self.MaxTargetsPerRow`))
      (if (>= (`self.LowerRowTargetsCount`) (`self.MaxTargetsPerRow`))
        (set `self.RowsFull` true :!label _label)
        (else
          (if (== (`KismetMathLibrary.RandomIntegerInRange` 0 1) 0) :!label _label_2
            (set `self.SpawnCoordinate` (`SceneComponent.K2_GetComponentLocation` (`self.Left Lower SpawnPoint`)))
            (set `self.FlippedDirection` false)
            (else
              (set `self.SpawnCoordinate` (`SceneComponent.K2_GetComponentLocation` (`self.Right Lower SpawnPoint`)))
              (set `self.FlippedDirection` true)))))
      (else
        (if (== (`KismetMathLibrary.RandomIntegerInRange` 0 1) 0) :!label _label_3
          (set `self.SpawnCoordinate` (`SceneComponent.K2_GetComponentLocation` (`self.Left Upper SpawnPoint`)))
          (set `self.FlippedDirection` false)
          (else
            (set `self.SpawnCoordinate` (`SceneComponent.K2_GetComponentLocation` (`self.Right Upper SpawnPoint`)))
            (set `self.FlippedDirection` true)))))
    (elif (>= (`self.LowerRowTargetsCount`) (`self.MaxTargetsPerRow`))
      (if (>= (`self.UpperRowTargetsCount`) (`self.MaxTargetsPerRow`))
        (goto _label)
        (else
          (goto _label_3)))
      (else
        (goto _label_2)))))

(fn `GetTimespanString`
  (params (InTimespan :type "Timespan Structure"))
  (returns (ReturnValue :type String))
  (bind (_days _hours _minutes _seconds _milliseconds) (`KismetMathLibrary.BreakTimespan` InTimespan))
  (return (`KismetStringLibrary.Concat_StrStr` (`KismetStringLibrary.Right` (`KismetStringLibrary.Concat_StrStr` "0" (`KismetStringLibrary.Conv_IntToString` _minutes)) 2) " : " (`KismetStringLibrary.Right` (`KismetStringLibrary.Concat_StrStr` "0" (`KismetStringLibrary.Conv_IntToString` _seconds)) 2) " : " (`KismetStringLibrary.Conv_IntToString` _milliseconds))))

(fn `UpdateNumberOfTargets`
  (set `self.UpperRowTargetsCount` (`KismetArrayLibrary.Array_Length` (`PrimitiveComponent.GetOverlappingActors` (`self.UpperTargetField`) "/Game/Targets/BP_Target.BP_Target_C")))
  (bind _output_get (set `self.LowerRowTargetsCount` (`KismetArrayLibrary.Array_Length` (`PrimitiveComponent.GetOverlappingActors` (`self.LowerTargetField`) "/Game/Targets/BP_Target.BP_Target_C")))))

(fn `UserConstructionScript`)
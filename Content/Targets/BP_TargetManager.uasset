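; Manager actor that spawns moving BP_Target actors into an upper and a lower row, with a looping timer started at BeginPlay.
; SpawnTarget counts targets overlapping each row's field, then picks a random row, falling back to the other if it has reached its cap.
; It spawns at that row's left or right point at random, flipping direction for right-side spawns, and skips spawning when both rows are full.
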(event `self.ReceiveBeginPlay`
  (`KismetSystemLibrary.K2_SetTimerDelegate` (`|CreateDelegate` :!event `SpawnTarget`) 4.0 true))

(event `SpawnTarget`
  (`self.UpdateNumberOfTargets`)
  (`self.ChooseSpawnPoint`)
  (if (not (`self.RowsFull`))
    (bind _returnvalue (`|SpawnActorFromClass` "/Game/Targets/BP_Target.BP_Target_C" (`KismetMathLibrary.MakeTransform` (`self.SpawnCoordinate`)) "Undefined" "OverrideRootScale" null null))
    (if (`self.FlippedDirection`)
      (`/Game/Targets/BP_Target.SwitchDirection` _returnvalue))))

(fn `ChooseSpawnPoint`
  (set `self.RowsFull` false)
  (if (== (`KismetMathLibrary.RandomIntegerInRange` 0 1) 0)
    (if (>= (`self.UpperTargetsCount`) (`self.MaxTargetsPerRow`))
      (if (>= (`self.LowerTargetsCount`) (`self.MaxTargetsPerRow`))
        (set `self.RowsFull` true :!label _label)
        (else
          (if (== (`KismetMathLibrary.RandomIntegerInRange` 0 1) 0) :!label _label_2
            (set `self.SpawnCoordinate` (`SceneComponent.K2_GetComponentLocation` (`self.Left Lower SpawnPoint`)))
            (set `self.FlippedDirection` false)
            (else
              (set `self.SpawnCoordinate` (`SceneComponent.K2_GetComponentLocation` (`self.Right Lower SpawnPoint`)))
              (set `self.FlippedDirection` true)))))
      (else
        (if (== (`KismetMathLibrary.RandomIntegerInRange` 0 1) 0) :!label _label_3
          (set `self.SpawnCoordinate` (`SceneComponent.K2_GetComponentLocation` (`self.Left Upper SpawnPoint`)))
          (set `self.FlippedDirection` false)
          (else
            (set `self.SpawnCoordinate` (`SceneComponent.K2_GetComponentLocation` (`self.Right Upper SpawnPoint`)))
            (set `self.FlippedDirection` true)))))
    (elif (>= (`self.LowerTargetsCount`) (`self.MaxTargetsPerRow`))
      (if (>= (`self.UpperTargetsCount`) (`self.MaxTargetsPerRow`))
        (goto _label)
        (else
          (goto _label_3)))
      (else
        (goto _label_2)))))

(fn `UpdateNumberOfTargets`
  (set `self.UpperTargetsCount` (`KismetArrayLibrary.Array_Length` (`PrimitiveComponent.GetOverlappingActors` (`self.UpperTargetField`) "/Game/Targets/BP_Target.BP_Target_C")))
  (bind _output_get (set `self.LowerTargetsCount` (`KismetArrayLibrary.Array_Length` (`PrimitiveComponent.GetOverlappingActors` (`self.LowerTargetField`) "/Game/Targets/BP_Target.BP_Target_C")))))

(fn `UserConstructionScript`)
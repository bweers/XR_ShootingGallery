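; BP_CoolwaterTrigger is a shootable-target style actor that opens MainLevel when its KnockDown event fires, ignoring the points flag.
; On BeginPlay it reverses a knock-down timeline from the end to animate its rotation.
; UpdatePosition and SwitchDirection support sideways movement, but the looping timer node is disconnected.
; The round-start, hit sound, collision-off and destroy logic is also left unconnected.
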(event `UpdatePosition`
  (`self.K2_AddActorWorldOffset` (* (`self.GetActorRightVector`) (`self.Speed`))))

(event `/Game/Targets/BPI_Targets.KnockDown`
  (params (CountsForPoints :type Boolean))
  (`GameplayStatics.OpenLevel` "MainLevel"))

(event `self.ReceiveBeginPlay`
  (bind (_direction _yrotation) (`Timeline|KnockDownAnimTimeline` :!via `ReverseFromEnd`)
    (:`Update`
      (`self.K2_SetActorRotation` (`KismetMathLibrary.MakeRotator` 0.0 _yrotation)))))

(fn `SwitchDirection`
  (set `self.Speed` (* (`self.Speed`) -1.0)))

(fn `UserConstructionScript`)
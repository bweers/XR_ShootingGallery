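; BP_Target is a moving shooting-gallery style target that awards points to its parent BP_TargetManager when knocked down.
; A looping timer set on BeginPlay drives sideways movement along its right vector, and SwitchDirection reverses it by negating Speed.
; KnockDown adds the score, disables collision, starts a timeline that tips the target over, and destroys the actor after a short delay.
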(event `self.ReceiveBeginPlay`
  (`KismetSystemLibrary.K2_SetTimerDelegate` (`|CreateDelegate` :!event `UpdatePosition`) 0.01 true))

(event `UpdatePosition`
  (`self.K2_AddActorWorldOffset` (* (`self.GetActorRightVector`) (`self.Speed`))))

(event `/Game/Targets/BPI_Targets.KnockDown`
  (`KismetSystemLibrary.PrintString` "HIT")
  (`|ExecutionSequence`
    (:`then_0`
      (bind _asbp_target_manager (cast `/Game/Targets/BP_TargetManager` (`self.GetParentActor`)))
      (`/Game/Targets/BP_TargetManager.AddPoints` _asbp_target_manager 300))
    (:`then_1`
      (`PrimitiveComponent.SetCollisionEnabled` (`self.Collider`) "NoCollision")
      (bind (_direction _yrotation) (`Timeline|KnockDownAnimTimeline`)
        (:`Update`
          (`self.K2_SetActorRotation` (`KismetMathLibrary.MakeRotator` 0.0 _yrotation)))))
    (:`then_2`
      (`KismetSystemLibrary.Delay` 0.2)
      (`self.K2_DestroyActor`))))

(fn `SwitchDirection`
  (set `self.Speed` (* (`self.Speed`) -1.0)))

(fn `UserConstructionScript`)